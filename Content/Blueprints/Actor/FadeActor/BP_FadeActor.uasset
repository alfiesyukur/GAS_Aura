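; BP_FadeActor is an actor whose mesh fades out and back in through a timeline-driven "Fade" material parameter.
; Construction creates dynamic instances from FadeMaterialInstances, which FadeOut assigns to the mesh slots before playing the timeline; Fadein reverses it.
; On finish, a fade value of one resets the mesh materials.
; If BlockVisibility is set, the mesh ignores the Visibility channel when faded to zero and blocks it again at one.
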(event `/Game/Blueprints/Actor/FadeActor/BP_FadeInterface.FadeOut`
  (`self.SetMaterialToDynamicInstance`)
  (bind (_direction _fade) (`Timeline|FadeOutMaterialTimeline` :!label _label)
    (:`Update`
      (for _array_element (`self.DynamicMaterialInstances`)
        (`MaterialInstanceDynamic.SetScalarParameterValue` _array_element "Fade" _fade)))
    (:`Finished`
      (`self.FadeFinished` _fade))))

(event `/Game/Blueprints/Actor/FadeActor/BP_FadeInterface.FadeIn`
  (goto _label :!via `Reverse`))

(fn `FadeFinished`
  (params (FadeAmount :type "Float (single-precision)"))
  (if (>= FadeAmount 1.0)
    (`self.ResetMaterials`)
    (if (`self.BlockVisibility`)
      (`PrimitiveComponent.SetCollisionResponseToChannel` (`self.Mesh`) "ECC_Visibility" "ECR_Block"))
    (elif (<= FadeAmount 0.0)
      (if (`self.BlockVisibility`)
        (`PrimitiveComponent.SetCollisionResponseToChannel` (`self.Mesh`) "ECC_Visibility" "ECR_Ignore")))))

(fn `ResetMaterials`
  (for (_ _array_index) (`self.OriginalMaterials`)
    (`PrimitiveComponent.SetMaterial` (`self.Mesh`) _array_index null)))

(fn `SetMaterialToDynamicInstance`
  (for (_array_element _array_index) (`self.DynamicMaterialInstances`)
    (`PrimitiveComponent.SetMaterial` (`self.Mesh`) _array_index _array_element)))

(fn `UserConstructionScript`
  (bind _dynamicmaterialinstances (`self.DynamicMaterialInstances`))
  (`KismetArrayLibrary.Array_Clear` (`self.DynamicMaterialInstances`))
  (`KismetArrayLibrary.Array_Clear` (`self.OriginalMaterials`))
  (set `self.OriginalMaterials` (`MeshComponent.GetMaterials` (`self.Mesh`)))
  (for _array_element (`self.FadeMaterialInstances`)
    (bind _returnvalue (`KismetMaterialLibrary.CreateDynamicMaterialInstance` _array_element))
    (`KismetArrayLibrary.Array_Add` _dynamicmaterialinstances _returnvalue)
    (`KismetSystemLibrary.LogString` (`KismetStringLibrary.Conv_IntToString` (`KismetArrayLibrary.Array_Length` _dynamicmaterialinstances)))))