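; GA_MeleeAttack is a gameplay ability that turns its avatar toward its combat target and performs a melee spear attack.
; It plays the spear attack montage while waiting for the Event.Montage.Melee gameplay event.
; On that event, it gathers live players in a small sphere around the combat socket, excluding the avatar, calls CauseDamage on each, then ends the ability.
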(event `self.K2_ActivateAbility`
  (bind _returnvalue (`self.GetAvatarActorFromActorInfo`))
  (bind _returnvalue_2 (`self.GetAvatarActorFromActorInfo`))
  (bind _returnvalue_3 (message `CombatInterface.GetCombatTarget` _returnvalue_2))
  (message `CombatInterface.UpdateFacingTarget` _returnvalue_2 (`Actor.K2_GetActorLocation` _returnvalue_3))
  (`AbilityTask_PlayMontageAndWait.CreatePlayMontageAndWaitProxy` "None" "/Game/Assets/Enemies/Goblin/Animations/Spear/AM_Attack_Spear.AM_Attack_Spear" 1.0 "None" true 1.0 0.0 true
    (:`then`
      (`AbilityTask_WaitGameplayEvent.WaitGameplayEvent` (struct :`TagName` "Event.Montage.Melee") null
        (:`EventReceived`
          (bind _returnvalue_4 (message `CombatInterface.GetCombatSocketLocation` _returnvalue))
          (bind _outoverlappingactors (`AuraAbilitySystemLibrary.GetLivePlayerWithRadius` _returnvalue (`|MakeArray` _returnvalue) 45.0 _returnvalue_4))
          (for _array_element _outoverlappingactors
            (`self.CauseDamage` _array_element))
          (`self.K2_EndAbility`))))))