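; Enemy ranged attack gameplay ability that turns the avatar toward its combat target and fires a projectile at it.
; It plays a random tagged attack montage and waits for a gameplay event matching that montage's socket tag.
; The event spawns the projectile at the target's current location, with optional pitch override, and ends the ability while the montage plays on.
; Debug spheres mark target and socket.
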(event `self.K2_ActivateAbility`
  (bind _returnvalue (`self.GetAvatarActorFromActorInfo`))
  (bind _returnvalue_2 (`self.GetAvatarActorFromActorInfo`))
  (bind (_taggedmontage_montage _taggedmontage_montagetag _taggedmontage_sockettag) (break `TaggedMontage` (`self.TaggedMontage`)))
  (bind _returnvalue_3 (message `EnemyInterface.GetCombatTarget` _returnvalue_2))
  (bind _returnvalue_4 (`Actor.K2_GetActorLocation` _returnvalue_3))
  (message `CombatInterface.UpdateFacingTarget` _returnvalue_2 _returnvalue_4)
  (`KismetSystemLibrary.DrawDebugSphere` _returnvalue_4 15.0 12 (struct :`R` 1.0 :`G` 0.74805 :`B` 0.020335 :`A` 1.0) 0.75)
  (bind _returnvalue_5 (message `CombatInterface.GetAttackMontages` (`self.GetAvatarActorFromActorInfo`)))
  (bind _output_get (set `self.TaggedMontage` (`self.GetRandomTaggedMontageFromArray` _returnvalue_5)))
  (`AbilityTask_PlayMontageAndWait.CreatePlayMontageAndWaitProxy` "None" (break `TaggedMontage` _output_get) 1.0 "None" false
    (:`then`
      (`AbilityTask_WaitGameplayEvent.WaitGameplayEvent` (`.SocketTag` (break `TaggedMontage` _output_get)) null true
        (:`then`
          (bind _returnvalue_6 (message `CombatInterface.GetCombatSocketLocation` _returnvalue (`.SocketTag` (break `TaggedMontage` _output_get))))
          (`KismetSystemLibrary.DrawDebugSphere` _returnvalue_6 12.0 12 (struct :`R` 1.0 :`G` 0.72552 :`B` 0.026042 :`A` 1.0) 0.35)
          (bind _returnvalue_7 (message `EnemyInterface.GetCombatTarget` _returnvalue))
          (`self.SpawnProjectile` (`Actor.K2_GetActorLocation` _returnvalue_7) _taggedmontage_sockettag (`self.ShouldOverridePitch`) (`self.PitchOverride`))
          (`self.K2_EndAbility`))))
    (:`OnCompleted`
      (`self.K2_EndAbility` :!label _label))
    (:`OnInterrupted`
      (goto _label))
    (:`OnCancelled`
      (goto _label))))