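; Enemy summon ability that spawns random minions with their default controllers, using the Shaman summon montage.
; On activation it faces the combat target and waits for the Abilities.Summon event while the montage plays.
; The event shuffles the spawn locations, plays ground Niagara effects at all of them, then spawns minions through a delayed loop, incrementing the owner's minion count.
; The ability ends when the loop finishes or the montage completes or aborts.
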(event `self.K2_ActivateAbility`
  (bind _returnvalue (`self.GetAvatarActorFromActorInfo`))
  (bind _returnvalue_2 (`self.GetAvatarActorFromActorInfo`))
  (bind _output (`|GetArrayItem` (`self.SpawnLocations`) (`self.SpawnLocationIndex`)))
  (bind _returnvalue_3 (+ _output (0.0 0.0 70.0)))
  (bind _returnvalue_4 (message `EnemyInterface.GetCombatTarget` _returnvalue))
  (bind _returnvalue_5 (`Actor.K2_GetActorLocation` _returnvalue_4))
  (message `CombatInterface.UpdateFacingTarget` _returnvalue _returnvalue_5)
  (`KismetSystemLibrary.DrawDebugSphere` _returnvalue_5 15.0 12 (struct :`R` 0.022275 :`G` 0.16805 :`B` 1.0 :`A` 1.0) 5.0 5.0)
  (`KismetArrayLibrary.Array_Clear` (`self.SpawnLocations`))
  (`AbilityTask_PlayMontageAndWait.CreatePlayMontageAndWaitProxy` "None" "/Game/Assets/Enemies/Shaman/Animations/AM_Shaman_Summon.AM_Shaman_Summon" 1.0 "None" false
    (:`then`
      (`AbilityTask_WaitGameplayEvent.WaitGameplayEvent` (struct :`TagName` "Abilities.Summon") null
        (:`EventReceived`
          (bind _returnvalue_6 (`self.GetSpawnLocations`))
          (bind _output_get (set `self.SpawnLocations` _returnvalue_6))
          (`KismetArrayLibrary.Array_Shuffle` _output_get)
          (for _array_element (`self.SpawnLocations`)
            (`NiagaraFunctionLibrary.SpawnSystemAtLocation` "/Game/Assets/Effects/Combat/NS_GroundSummon.NS_GroundSummon" _array_element))
          (if (< (`self.SpawnLocationIndex`) (`KismetArrayLibrary.Array_Length` (`self.SpawnLocations`))) :!label _label
            (`KismetSystemLibrary.DrawDebugSphere` _output 25.0 12 (struct :`R` 1.0 :`G` 0.668679 :`A` 1.0) 0.8)
            (bind _aspawn (cast `Pawn` _returnvalue_2))
            (bind _returnvalue_7 (`|SpawnActorFromClass` (`self.GetRandomMinionClass`) (`KismetMathLibrary.MakeTransform` _returnvalue_3 (`KismetMathLibrary.FindLookAtRotation` (`Actor.K2_GetActorLocation` _returnvalue_2) _returnvalue_3)) "AlwaysSpawn" "MultiplyWithRoot" _returnvalue_2 _aspawn))
            (`Pawn.SpawnDefaultController` _returnvalue_7)
            (`/Engine/EditorBlueprintResources/StandardMacros.IncrementInt` (`self.SpawnLocationIndex`)
              (:`  `
                (message `CombatInterface.IncrementMinionCount` (`self.GetAvatarActorFromActorInfo`) 1)
                (`KismetSystemLibrary.Delay` 0.25)
                (goto _label)))
            (else
              (`self.K2_EndAbility`))))))
    (:`OnCompleted`
      (`self.K2_EndAbility` :!label _label_2))
    (:`OnInterrupted`
      (goto _label_2))
    (:`OnCancelled`
      (goto _label_2))))