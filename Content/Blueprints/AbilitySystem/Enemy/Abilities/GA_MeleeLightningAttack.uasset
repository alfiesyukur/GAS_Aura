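; Enemy gameplay ability that performs a melee lightning attack against players.
; It faces the combat target, plays a random tagged attack montage and waits for that montage's gameplay event.
; The event runs a small radius check at the tagged combat socket, damaging non-friendly live players and firing blood and melee impact cue effects.
; The ability ends after the check, letting the montage play on, and a debug sphere marks the hit point.
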(event `self.K2_ActivateAbility`
  (bind _returnvalue (`self.GetAvatarActorFromActorInfo`))
  (bind _returnvalue_2 (`self.GetAvatarActorFromActorInfo`))
  (bind (_taggedmontage_montage _taggedmontage_montagetag _taggedmontage_sockettag) (break `TaggedMontage` (`self.TaggedMontage`)))
  (bind (_taggedmontage_montage_2 _taggedmontage_montagetag_2) (break `TaggedMontage` (`self.TaggedMontage`)))
  (set `self.HasHitTarget` false)
  (bind _returnvalue_3 (message `EnemyInterface.GetCombatTarget` _returnvalue))
  (set `self.CombatTarget` _returnvalue_3)
  (message `CombatInterface.UpdateFacingTarget` _returnvalue (`Actor.K2_GetActorLocation` _returnvalue_3))
  (bind _returnvalue_4 (message `CombatInterface.GetAttackMontages` _returnvalue))
  (bind _output_get (set `self.TaggedMontage` (`self.GetRandomTaggedMontageFromArray` _returnvalue_4)))
  (`AbilityTask_PlayMontageAndWait.CreatePlayMontageAndWaitProxy` "None" (break `TaggedMontage` _output_get) 1.0 "None" false 1.0 0.0 true
    (:`then`
      (`AbilityTask_WaitGameplayEvent.WaitGameplayEvent` _taggedmontage_montagetag null
        (:`EventReceived`
          (bind _output_get_2 (set `self.AvatarFromActorInfo` _returnvalue_2))
          (bind _returnvalue_5 (message `CombatInterface.GetCombatSocketLocation` _output_get_2 _taggedmontage_sockettag))
          (bind _output_get_3 (set `self.CombatSocketLocation` _returnvalue_5))
          ;[1 1 1] Debug Sphere.
          (`KismetSystemLibrary.DrawDebugSphere` (`self.CombatSocketLocation`) 8.0 12 (struct :`R` 0.121892 :`G` 1.0 :`A` 1.0) 0.75 2.0)
          (bind _outoverlappingactors (`AuraAbilitySystemLibrary.GetLivePlayersWithinRadius` (`self.AvatarFromActorInfo`) (`|MakeArray` _returnvalue_2) 50.0 _output_get_3))
          (for _array_element _outoverlappingactors
            (if (`AuraAbilitySystemLibrary.IsNotFriend` (`self.AvatarFromActorInfo`) _array_element)
              (`self.CauseMeleeDamage` _array_element (`self.CombatSocketLocation`))
              (set `self.HasHitTarget` true)
              (message `CombatInterface.GetBloodEffect` _array_element)
              (`self.K2_ExecuteGameplayCueWithParams` (struct :`TagName` "GameplayCue.MeleeImpact") (`AbilitySystemBlueprintLibrary.MakeGameplayCueParameters` 0.0 0.0 (struct) (struct :`TagName` "GameplayCue.MeleeImpact") (struct) (`BlueprintGameplayTagLibrary.MakeGameplayTagContainerFromTag` _taggedmontage_montagetag_2) (struct) (`self.CombatSocketLocation`) (0.0 0.0 0.0) (`self.CombatTarget`) (`self.AvatarFromActorInfo`)))
              (`self.K2_EndAbility`)))
          (`self.K2_EndAbility`))))
    (:`OnCompleted`
      (`self.K2_EndAbility` :!label _label))
    (:`OnInterrupted`
      (goto _label))
    (:`OnCancelled`
      (goto _label))))