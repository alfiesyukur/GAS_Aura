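; Electrocute gameplay ability: a held-input lightning beam from the caster's weapon toward the target under the mouse.
; It commits on valid target data, turns the caster, plays a montage, and on its gameplay event traces the first target and locks movement.
; A looping ShockLoop cue sits on a CombatInterface target, or on the caster otherwise.
; Input release removes the cue, restores movement and cursor, and ends the ability.
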(event `self.K2_ActivateAbility`
  (bind _returnvalue (`self.GetAvatarActorFromActorInfo`))
  (set `self.MouseHitActor` null)
  (set `self.MouseHitLocation` (0.0 0.0 0.0))
  (message `CombatInterface.SetInShockLoop` _returnvalue false)
  (if (`KismetSystemLibrary.DoesImplementInterface` _returnvalue "/Script/Aura.CombatInterface")
    ;[1 0.3953 0.5054] Store Mouse data Variables
    (bind (_asynctaskproxy _datahandle) (`TargetDataUnderMouse.CreateTargetDataUnderMouse`)
      (:`ValidData`
        (bind _returnvalue_2 (`AbilitySystemBlueprintLibrary.GetHitResultFromTargetData` _datahandle))
        (bind (_bblockinghit _binitialoverlap _time _distance _location _impactpoint _normal _impactnormal _physmat _hitactor) (`GameplayStatics.BreakHitResult` _returnvalue_2))
        (if (or _bblockinghit (`KismetSystemLibrary.IsValid` _hitactor))
          (`self.StoreMousedataInfo` _returnvalue_2)
          (`self.StoreOwnerVariables`)
          (`|ExecutionSequence`
            (:`then_0`
              (`self.K2_CommitAbility`)
              (`AbilityTask_WaitInputPress.WaitInputPress` false
                (:`then`
                  (set `PlayerController.bShowMouseCursor` false (`self.OwnerPlayerController`))
                  (message `CombatInterface.UpdateFacingTarget` (`self.GetAvatarActorFromActorInfo`) (`self.MouseHitLocation`))
                  (`self.K2_ExecuteGameplayCue` (struct :`TagName` "GameplayCue.ShockBurst"))
                  (`AbilityTask_PlayMontageAndWait.CreatePlayMontageAndWaitProxy` "None" (`self.Montage_Electrocute`) 1.0 "None" false
                    (:`then`
                      (`AbilityTask_WaitGameplayEvent.WaitGameplayEvent` (struct :`TagName` "Event.Montage.Electrocute") null true
                        (:`EventReceived`
                          (`self.SpawnElectricBeam`)
                          (`self.FreezeActor`))))))))
            (:`then_1`
              (`AbilityTask_WaitInputRelease.WaitInputRelease` false
                (:`OnRelease`
                  (`self.PrepareToEndAbility`)
                  (`self.UnfreezeActor`)
                  (`self.K2_EndAbility`)))))
          (else
            (`self.K2_EndAbility`)))))))

(event `self.K2_OnEndAbility`
  (params (bWasCancelled :type Boolean))
  (message `CombatInterface.SetInShockLoop` (`self.GetAvatarActorFromActorInfo`) false))

(fn `FreezeActor`
  (message `CombatInterface.SetInShockLoop` (`self.GetAvatarActorFromActorInfo`) true)
  (`CharacterMovementComponent.DisableMovement` (`Character.CharacterMovement` (`self.OwnerCharacter`)))
  (return))

(fn `PrepareToEndAbility`
  (if (`self.FirstTargetImplementInterface`)
    (`GameplayCueFunctionLibrary.RemoveGameplayCueOnActor` (`self.MouseHitActor`) (struct :`TagName` "GameplayCue.ShockLoop") (`self.FirstTargetQueParams`))
    (else
      (`GameplayCueFunctionLibrary.RemoveGameplayCueOnActor` (`self.GetAvatarActorFromActorInfo`) (struct :`TagName` "GameplayCue.ShockLoop") (`self.FirstTargetQueParams`))))
  (return))

(fn `SpawnElectricBeam`
  (locals (QueTarget :type "Actor Object Reference"))
  (`self.TraceFirstTarget` (`self.MouseHitLocation`))
  (bind _returnvalue (message `CombatInterface.GetWeapon` (`self.OwnerCharacter`)))
  (set `self.FirstTargetQueParams` (`AbilitySystemBlueprintLibrary.MakeGameplayCueParameters` 0.0 0.0 (struct) (struct) (struct) (struct) (struct) (`self.MouseHitLocation`) (0.0 0.0 0.0) null null (`self.MouseHitActor`) null 1 1 _returnvalue))
  ;[1 1 1] Is Mouse Hit Actor an Enemy.
  (bind _output_get (set `self.FirstTargetImplementInterface` (`KismetSystemLibrary.DoesImplementInterface` (`self.MouseHitActor`) "/Script/Aura.CombatInterface")))
  (if _output_get
    (set `local.QueTarget` (`self.MouseHitActor`))
    (else
      (set `local.QueTarget` (`self.GetAvatarActorFromActorInfo`))))
  (`GameplayCueFunctionLibrary.AddGameplayCueOnActor` (`local.QueTarget`) (struct :`TagName` "GameplayCue.ShockLoop") (`self.FirstTargetQueParams`)))

(fn `UnfreezeActor`
  (set `PlayerController.bShowMouseCursor` true (`self.OwnerPlayerController`))
  (`CharacterMovementComponent.SetMovementMode` (`Character.CharacterMovement` (`self.OwnerCharacter`)) "MOVE_Walking" 0)
  (return))