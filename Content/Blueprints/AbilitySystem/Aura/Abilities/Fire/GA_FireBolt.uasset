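; GA_FireBolt is Aura's Fire Bolt gameplay ability, firing homing-target projectiles at the point or actor under the mouse.
; It waits for mouse target data, commits only on a valid hit, and turns the caster toward the target via the combat interface.
; A cast montage's gameplay event triggers SpawnProjectiles from the weapon socket with an overridden pitch.
; The ability ends when the montage finishes or the hit is invalid.
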(event `self.K2_ActivateAbility`
  (bind (_asynctaskproxy _datahandle) (`TargetDataUnderMouse.CreateTargetDataUnderMouse`)
    (:`ValidData`
      (bind (_bblockinghit _binitialoverlap _time _distance _location _impactpoint _normal _impactnormal _physmat _hitactor) (`GameplayStatics.BreakHitResult` (`AbilitySystemBlueprintLibrary.GetHitResultFromTargetData` _datahandle)))
      (bind _output_get (set `self.MouseHitActor` _hitactor))
      (if (or (`KismetSystemLibrary.IsValid` _output_get) _bblockinghit)
        (`self.K2_CommitAbility`)
        (bind _output_get_2 (set `self.ProjectileTargetLocation` _location))
        (bind _ascombat_interface (cast `CombatInterface` (`self.GetAvatarActorFromActorInfo`)))
        (`CombatInterface.UpdateFacingTarget` _ascombat_interface _output_get_2)
        (`AbilityTask_PlayMontageAndWait.CreatePlayMontageAndWaitProxy` "None" "/Game/Assets/Characters/Aura/Animations/Abilities/AM_Cast_FireBolt_Aura.AM_Cast_FireBolt_Aura" 1.0 "None" false
          (:`then`
            (`AbilityTask_WaitGameplayEvent.WaitGameplayEvent` (struct :`TagName` "Event.Montage.FireBolt") null
              (:`EventReceived`
                (`self.SpawnProjectiles` (`self.ProjectileTargetLocation`) (`BlueprintGameplayTagLibrary.MakeLiteralGameplayTag` (struct :`TagName` "CombatSocket.Weapon")) true 55.0 (`self.MouseHitActor`)))))
          (:`OnCompleted`
            (`self.K2_EndAbility` :!label _label))
          (:`OnBlendOut`
            (goto _label))
          (:`OnInterrupted`
            (goto _label))
          (:`OnCancelled`
            (goto _label)))
        (else
          (`self.K2_EndAbility`))))))